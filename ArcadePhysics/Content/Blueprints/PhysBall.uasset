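; PhysBall is a physics-driven ball actor that can be pushed, kicked, stopped and reset.
; On BeginPlay it stores its start location, and ResetBall teleports it back there with a random launch velocity and a new random Force vector.
; Tick adds that constant force while ShouldApplyForce is set, without scaling by DeltaTime.
; Separate events apply a random impulse or zero the linear velocity.
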(event `self.ReceiveBeginPlay`
  ;[1 1 1] Store the initial location
  (set `self.Initial Location` (`self.K2_GetActorLocation`))
  (`self.Reset Ball`))

(event `Reset Ball`
  ;[1 1 1] Reset the Linear Velocity to a random direction
  (`PrimitiveComponent.SetPhysicsLinearVelocity` (`self.Physics Body`) (* (`KismetMathLibrary.RandomUnitVector`) (`self.Initial Speed`)) false "None")
  ;[1 1 1] Move the ball back to its initial location
  (`self.K2_SetActorLocation` (`self.Initial Location`) false true)
  ;[1 1 1] Calculate a random force
  (set `self.Force` (* (`KismetMathLibrary.RandomUnitVector`) (`self.Force Magnitude`))))

(event `self.ReceiveTick`
  (params (DeltaSeconds :type "Float (single-precision)"))
  ;[1 1 1] Check if we should apply force this frame
  (if (`self.Should Apply Force`)
    ;[1 1 1] Apply the force. Do not multiply by DeltaTime
    (`PrimitiveComponent.AddForce` (`self.Physics Body`) (`self.Force`) "None" false)))

(event `Apply Random Impulse`
  ;[1 1 1] Apply a random impulse to the ball
  (`PrimitiveComponent.AddImpulse` (`self.Physics Body`) (* (`KismetMathLibrary.RandomUnitVector`) 1000.0) "None" false))

(event `Zero Out Velocity`
  ;[1 1 1] Set the linear velocity to zero
  (`PrimitiveComponent.SetPhysicsLinearVelocity` (`self.Physics Body`) (0.0 0.0 0.0) false "None"))

(fn `UserConstructionScript`)